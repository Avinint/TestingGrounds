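; AI controller for guard NPCs that runs the GuardBehavior behavior tree on the PatrolData blackboard.
; AI perception writes sensed actors lacking the "Enemy" tag to the EnemyKey blackboard value and clears it when such an actor is no longer sensed.
; Each tick sets the controlled Guard's Aiming and Shooting flags according to whether the controller has a valid focus actor.
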(event OnTargetPerceptionUpdated(AIPerception)
  (params (Actor :type Actor%20Object%20Reference) (Stimulus :type AI%20Stimulus%20Structure))
  (bind _enemykey (Variables|Default|GetEnemyKey))
  (if (not (Actor|ActorHasTag Actor "Enemy"))
    (if (.bSuccessfullySensed (Utilities|Struct|BreakAIStimulus Stimulus))
      (AI|Components|Blackboard|SetValueasObject (stale EventBeginPlay _blackboardcomponent) _enemykey Actor)
      (else
        (AI|Components|Blackboard|ClearValue (stale EventBeginPlay _blackboardcomponent) _enemykey)))))

(event EventBeginPlay
  (bind _blackboardcomponent (Class|AIController|UseBlackboard "/Game/Dynamic/NPC/AI/PatrolData.PatrolData"))
  (AI|RunBehaviorTree "/Game/Dynamic/NPC/AI/GuardBehavior.GuardBehavior"))

(event EventTick
  (params (DeltaSeconds :type Float%20%28single-precision%29))
  (bind _returnvalue (Class|AIController|GetFocusActor))
  (bind _returnvalue_2 (Utilities|IsValid _returnvalue))
  (bind _asguard (Utilities|Casting|CastToGuard (Pawn|GetControlledPawn)))
  (Variables|/Game/Dynamic/NPC/Behavior/Guard.Guard_C|SetAiming _asguard _returnvalue_2)
  (Variables|/Game/Dynamic/NPC/Behavior/Guard.Guard_C|SetShooting _asguard _returnvalue_2))

(fn ConstructionScript)