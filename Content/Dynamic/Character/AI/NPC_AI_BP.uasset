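; AI controller for guard NPCs that starts the PatrolData blackboard and runs the GuardBehavior behavior tree on BeginPlay.
; AI Perception updates feed UpdateEnemyBlackboardKey, which ignores actors tagged "Enemy".
; Any other actor is written to the blackboard's EnemyKey when successfully sensed, and the key is cleared when that sensing fails.
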(event OnTargetPerceptionUpdated(AIPerception)
  (params (Actor :type Actor%20Object%20Reference) (Stimulus :type AI%20Stimulus%20Structure))
  (CallFunction|UpdateEnemyBlackboardKey Stimulus Actor Actor))

(event EventBeginPlay
  (Class|AIController|UseBlackboard "/Game/Dynamic/Character/AI/PatrolData.PatrolData")
  (AI|RunBehaviorTree "/Game/Dynamic/Character/AI/GuardBehavior.GuardBehavior"))

(fn ConstructionScript)

(fn UpdateEnemyBlackboardKey
  (params (AIStimulus :type AI%20Stimulus%20Structure%20%28by%20ref%29) (ObjectValue :type Object%20Object%20Reference) (self2 :type Actor%20Object%20Reference))
  (bind _returnvalue (AI|GetBlackboard 0))
  (bind _enemykey (Variables|Default|GetEnemyKey))
  (if (not (Actor|ActorHasTag self2 "Enemy"))
    (if (.bSuccessfullySensed (Utilities|Struct|BreakAIStimulus AIStimulus))
      (AI|Components|Blackboard|SetValueasObject _returnvalue _enemykey ObjectValue)
      (else
        (AI|Components|Blackboard|ClearValue _returnvalue _enemykey)))))